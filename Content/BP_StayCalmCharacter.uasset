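; StayCalm character Blueprint that drives a screen blur reflecting the character's panic level.
; The UpdatePanicBlur event maps a level from clear to strongest through chained branches, replacing the PanicPostProcess settings at each step.
; The blur comes from depth of field, with aperture and focal distance shrinking as panic rises.
; BeginPlay, Tick, overlap and construction logic are empty.
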(event `self.updatePanicBlur`
  (params (level :type Integer))
  ;[1 1 1] Level 0 Blur effect - Clear blur effect
  (if (== level 0)
    (set `PostProcessComponent.Settings` (make `PostProcessSettings` :`DepthOfFieldFstop` 1000.0 :`DepthOfFieldFocalDistance` 1000.0) (`self.PanicPostProcess`))
    (else
      ;[1 1 1] Level 1 Blur effect
      (if (== level 1)
        (set `PostProcessComponent.Settings` (make `PostProcessSettings` :`DepthOfFieldFstop` 5.0 :`DepthOfFieldFocalDistance` 30.0) (`self.PanicPostProcess`))
        (else
          ;[1 1 1] Level 2 blur effect
          (if (== level 2)
            (set `PostProcessComponent.Settings` (make `PostProcessSettings` :`DepthOfFieldFocalDistance` 20.0) (`self.PanicPostProcess`))
            (else
              ;[1 1 1] Level 3 Blur effect
              (if (== level 3)
                (set `PostProcessComponent.Settings` (make `PostProcessSettings` :`DepthOfFieldFstop` 3.0 :`DepthOfFieldFocalDistance` 15.0) (`self.PanicPostProcess`))))))))))

(fn `UserConstructionScript`)